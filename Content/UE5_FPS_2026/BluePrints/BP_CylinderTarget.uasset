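; BP_CylinderTarget is a moving shooting target that explodes on the second projectile hit.
; Tick moves it along the normalized Direction at Speed, while a looping timer flips Direction every TimeToChange seconds so it travels back and forth.
; The first BP_FirstPersonProjectile hit turns it red and sets Primed; a hit while primed plays explosion sound and particles, then destroys the actor.
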(event Custom|ChangeDirection
  (Variables|Default|SetDirection (* (Variables|Default|GetDirection) -1.0)))

(event EventBeginPlay
  (Utilities|Time|SetTimerbyEvent (delegate Custom|ChangeDirection) (Variables|Default|GetTimeToChange) true))

(event Collision|EventActorBeginOverlap
  (params (OtherActor :type Actor%20Object%20Reference)))

(event EventTick
  (params (DeltaSeconds :type Float%20%28single-precision%29))
  (Transformation|AddActorWorldOffset (* (Math|Vector|Normalize (Variables|Default|GetDirection)) (* (Variables|Default|GetSpeed) (Utilities|Time|GetWorldDeltaSeconds)))))

(event Collision|EventHit
  (params (MyComp :type Primitive%20Component%20Object%20Reference) (Other :type Actor%20Object%20Reference) (OtherComp :type Primitive%20Component%20Object%20Reference) (bSelfMoved :type Boolean) (HitLocation :type Vector :default "0, 0, 0") (HitNormal :type Vector :default "0, 0, 0") (NormalImpulse :type Vector :default "0, 0, 0") (Hit :type Hit%20Result%20Structure%20%28by%20ref%29))
  ;[1 1 1] 총알에 맞으면 머테리얼 변환
  (Utilities|Casting|CastToBP_FirstPersonProjectile Other)
  (if (Variables|Default|GetPrimed)
    (Audio|PlaySoundatLocation "/Game/StarterContent/Audio/Explosion01.Explosion01" HitLocation "0, 0, 0" 1.0 1.0 0.0 0 0 0 0)
    (Effects|SpawnEmitteratLocation "/Game/StarterContent/Particles/P_Explosion.P_Explosion" HitLocation)
    (Actor|DestroyActor)
    (else
      (Rendering|Material|SetMaterial (Variables|Debug|GetStaticMeshComponent) 0 "/Game/UE5_FPS_2026/Materials/M_TargetRed.M_TargetRed")
      (Variables|Default|SetPrimed true))))

(fn ConstructionScript)