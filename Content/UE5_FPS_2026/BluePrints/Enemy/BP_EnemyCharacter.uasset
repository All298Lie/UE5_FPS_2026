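; BP_EnemyCharacter is an enemy character that patrols back and forth between two patrol point actors.
; It starts toward the first point and switches its target to the other point whenever it overlaps the current one.
; Each change is written to the AI Blackboard as an object value under a configurable key, presumably for the behavior tree to drive movement.
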(event EventBeginPlay
  (Variables|AI|SetCurrentPatrolPoint (Variables|AI|GetPatrolPoint1))
  (Utilities|UpdatePatrolPointBB))

(event Collision|EventActorBeginOverlap
  (params (OtherActor :type Actor%20Object%20Reference))
  (if (== OtherActor (Variables|AI|GetPatrolPoint1))
    (Variables|AI|SetCurrentPatrolPoint (Variables|AI|GetPatrolPoint2))
    (Utilities|UpdatePatrolPointBB :!label _label)
    (elif (== OtherActor (Variables|AI|GetPatrolPoint2))
      (Variables|AI|SetCurrentPatrolPoint (Variables|AI|GetPatrolPoint1))
      (goto _label))))

(event EventTick
  (params (DeltaSeconds :type Float%20%28single-precision%29)))

(fn ConstructionScript
  (|CallParentFunction))